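; Player Bomberman character that moves tile by tile on the game mode's Map and drops bombs at its current cell.
; Direction input picks the next empty neighbor tile; Tick steers toward it with movement input, snapping to the tile center when stopping or turning.
; Power-up overlaps register with the GameInstance, and damage goes to HealthComponent.
; Death changes game state and enables mesh physics; destruction notifies the game mode.
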(event OnDeath(HealthComponent)
  (Default|SetState (Variables|Default|GetGameInstance) "NewEnumerator7")
  (Physics|SetSimulatePhysics (Variables|Character|GetMesh) true))

(event Game|Damage|EventAnyDamage
  (params (Damage :type Float%20%28single-precision%29) (DamageType :type Damage%20Type%20Object%20Reference) (InstigatedBy :type Controller%20Object%20Reference) (DamageCauser :type Actor%20Object%20Reference))
  (Default|OnTakeDamageEvent (Variables|Default|GetHealthComponent) Damage DamageType InstigatedBy DamageCauser))

(event EventDestroyed
  (bind _asbomber_man_game (Utilities|Casting|CastToBomberManGame (Game|GetGameMode)))
  (Default|OnBombermanDestroyedEvent _asbomber_man_game self))

(event EventBeginPlay
  (bind _asbomberman_game_instance (Utilities|Casting|CastToBombermanGameInstance (Game|GetGameInstance)))
  (Variables|Default|SetGameInstance _asbomberman_game_instance)
  (bind _asbomber_man_game (Utilities|Casting|CastToBomberManGame (Game|GetGameMode)))
  (Variables|Default|SetMap (Variables|/Game/Blueprints/BomberManGame.BomberManGame_C|GetMap _asbomber_man_game))
  (CallFunction|InitPositions))

(event Collision|EventActorBeginOverlap
  (params (OtherActor :type Actor%20Object%20Reference))
  (bind _aspower_up_interface (Utilities|Casting|CastToPowerUpInterface OtherActor))
  (bind _type (Default|GetPowerUpType _aspower_up_interface))
  (bind _asbomberman_game_instance (Utilities|Casting|CastToBombermanGameInstance (Game|GetGameInstance)))
  (Default|AddPowerUp _asbomberman_game_instance _type))

(event EventTick
  (params (DeltaSeconds :type Float%20%28single-precision%29))
  (CallFunction|UpdateMovement)
  (CallFunction|UpdateCurentPosition))

(event Input|ActionEvents|InputActionRight
  (params (Key :type Key%20Structure :default "AnyKey"))
  (:Pressed
    (Variables|Default|SetIsRightPressed true)
    (Variables|Default|SetTargetMovementDirection "NewEnumerator1"))
  (:Released
    (Variables|Default|SetIsRightPressed false)))

(event Input|ActionEvents|InputActionFire
  (params (Key :type Key%20Structure :default "AnyKey"))
  (:Pressed
    (Default|SpawnBomb (Variables|Default|GetMap) (Variables|Default|GetCurrentPosition))))

(event Input|ActionEvents|InputActionLeft
  (params (Key :type Key%20Structure :default "AnyKey"))
  (:Pressed
    (Variables|Default|SetIsLeftPressed true)
    (Variables|Default|SetTargetMovementDirection "NewEnumerator0"))
  (:Released
    (Variables|Default|SetIsLeftPressed false)))

(event Input|ActionEvents|InputActionDown
  (params (Key :type Key%20Structure :default "AnyKey"))
  (:Pressed
    (Variables|Default|SetIsDownPressed true)
    (Variables|Default|SetTargetMovementDirection "NewEnumerator3"))
  (:Released
    (Variables|Default|SetIsDownPressed false)))

(event Input|ActionEvents|InputActionUp
  (params (Key :type Key%20Structure :default "AnyKey"))
  (:Pressed
    (Variables|Default|SetIsUpPressed true)
    (Variables|Default|SetTargetMovementDirection "NewEnumerator2"))
  (:Released
    (Variables|Default|SetIsUpPressed false)))

(fn ConstructionScript)

(fn UpdateMovement
  (bind _targetposition (Variables|Default|GetTargetPosition))
  (bind _targetposition_2 (Variables|Default|GetTargetPosition))
  (bind _map (Variables|Default|GetMap))
  (bind _map_2 (Variables|Default|GetMap))
  (bind _targetposition_3 (Variables|Default|GetTargetPosition))
  (bind _map_3 (Variables|Default|GetMap))
  (bind _result (Default|ToWorldPosition _map _targetposition))
  (bind _result_2 (Default|ToWorldPosition _map_3 _targetposition_3))
  (bind _result_3 (Default|ToWorldPosition _map_2 _targetposition_2))
  (bind (_x _y) (Math|Vector|BreakVector _result))
  (bind (_x_2 _y_2) (Math|Vector|BreakVector _result_2))
  (bind (_x_3 _y_3) (Math|Vector|BreakVector _result_3))
  ;[1 1 1] Are we walking?
  (if (CallFunction|IsatTargetPosition)
    (Variables|Default|SetLastPosition (Variables|Default|GetTargetPosition))
    (if (CallFunction|IsMoveKeyPressed)
      (if (Utilities|Enum|Equal(Enum) (Variables|Default|GetCurrentMovementDirection) (Variables|Default|GetTargetMovementDirection))
        _
        (else
          (Transformation|SetActorLocation (Math|Vector|MakeVector _x_3 _y_3 (.Z (Math|Vector|BreakVector (Transformation|GetActorLocation)))) false false)
          (Components|Movement|StopMovementImmediately (Variables|Character|GetCharacterMovement))))
      ;[1 1 1] Change Target Position
      (CallFunction|UpdateTargetPosition)
      (Variables|Default|SetCurrentMovementDirection (Variables|Default|GetTargetMovementDirection))
      (if (CallFunction|Equal (Variables|Default|GetTargetPosition) (Variables|Default|GetLastPosition))
        (Components|Movement|StopMovementImmediately (Variables|Character|GetCharacterMovement))
        (Transformation|SetActorLocation (Math|Vector|MakeVector _x_2 _y_2 (.Z (Math|Vector|BreakVector (Transformation|GetActorLocation)))) false false)
        (else
          (CallFunction|Move)))
      (else
        (Components|Movement|StopMovementImmediately (Variables|Character|GetCharacterMovement))
        (Transformation|SetActorLocation (Math|Vector|MakeVector _x _y (.Z (Math|Vector|BreakVector (Transformation|GetActorLocation)))) false false)))
    (else
      (CallFunction|Move))))

(fn UpdateCurentPosition
  (bind _returnvalue (Transformation|GetActorLocation))
  (bind (_x _y) (Math|Vector|BreakVector _returnvalue))
  (Variables|Default|SetCurrentPosition (Default|ToLocalPosition (Variables|Default|GetMap) (Utilities|Struct|MakePosition2D (Math|Float|Truncate _x) (Math|Float|Truncate _y)))))

(fn InitPositions
  (CallFunction|UpdateCurentPosition)
  (Variables|Default|SetLastPosition (Variables|Default|GetCurrentPosition))
  (Variables|Default|SetTargetPosition (Variables|Default|GetCurrentPosition)))

(fn UpdateTargetPosition
  (bind _result (CallFunction|Position2d+Position2d (Variables|Default|GetLastPosition) (CallFunction|GetDirectionVector (Variables|Default|GetTargetMovementDirection))))
  (bind _result_2 (Default|IsEmpty (Variables|Default|GetMap) _result))
  (if _result_2
    (Variables|Default|SetTargetPosition _result)))

(fn IsatTargetPosition
  (bind _returnvalue (Transformation|GetActorLocation))
  (bind _targetposition (Variables|Default|GetTargetPosition))
  (bind _map (Variables|Default|GetMap))
  (bind _result (Default|ToWorldPosition _map _targetposition))
  (bind (_x _y) (Math|Vector|BreakVector _result))
  (return (Math|Vector|Equal(Vector) (Math|Vector|MakeVector _x _y (.Z (Math|Vector|BreakVector _returnvalue))) _returnvalue 1e+01)))

(fn Move
  (bind _returnvalue (Transformation|GetActorLocation))
  (bind _map (Variables|Default|GetMap))
  (bind _targetposition (Variables|Default|GetTargetPosition))
  (bind _result (Default|ToWorldPosition _map _targetposition))
  (bind _returnvalue_2 (- _result _returnvalue))
  (bind (_x _y) (Math|Vector|BreakVector _returnvalue_2))
  (Pawn|Input|AddMovementInput (Math|Vector|Normalize (Math|Vector|MakeVector _x _y 0.0)) 1.0 false))

(fn IsMoveKeyPressed
  (return (Math|Boolean|ORBoolean (Variables|Default|GetIsUpPressed) (Variables|Default|GetIsDownPressed) (Variables|Default|GetIsLeftPressed) (Variables|Default|GetIsRightPressed))))