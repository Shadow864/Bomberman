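; GodPlayerController is a player controller that relays the player's input to an AI controller as action calls.
; Tick polls the four arrow keys and calls the matching directional action each frame a key is held, while the Fire input action triggers ActionFire on press.
; SetAIController assigns the target controller, and every relay checks that it is valid first.
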(event EventTick
  (params (DeltaSeconds :type Float%20%28single-precision%29))
  ;[1 1 1] Movement
  (Utilities|FlowControl|Sequence
    (:then_0
      (if (Game|Player|IsInputKeyDown "Up")
        (if (Utilities|IsValid (Variables|Default|GetAiController))
          (Default|ActionUp (Variables|Default|GetAiController)))))
    (:then_1
      (if (Game|Player|IsInputKeyDown "Down")
        (if (Utilities|IsValid (Variables|Default|GetAiController))
          (Default|ActionDown (Variables|Default|GetAiController)))))
    (:then_2
      (if (Game|Player|IsInputKeyDown "Left")
        (if (Utilities|IsValid (Variables|Default|GetAiController))
          (Default|ActionLeft (Variables|Default|GetAiController)))))
    (:then_3
      (if (Game|Player|IsInputKeyDown "Right")
        (if (Utilities|IsValid (Variables|Default|GetAiController))
          (Default|ActionRight (Variables|Default|GetAiController)))))))

(event Input|ActionEvents|InputActionFire
  (params (Key :type Key%20Structure :default "AnyKey"))
  ;[1 1 1] Action
  (:Pressed
    (if (Utilities|IsValid (Variables|Default|GetAiController))
      (Default|ActionFire (Variables|Default|GetAiController)))))

(fn ConstructionScript)

(fn SetAIController
  (params (AiController :type Bomber%20Man%20AI%20Controller%20Object%20Reference))
  (Variables|Default|SetAiController AiController))