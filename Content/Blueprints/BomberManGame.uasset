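; BomberManGame is a Bomberman game-level Blueprint that reacts to the creation and destruction of bombs and Bomberman characters.
; Bomb events maintain a live bomb count.
; When a Bomberman is created, it gives that character's AI controller to player 0's GodPlayerController and passes it the Map, drawing debug text if either cast fails.
; When a Bomberman is destroyed, it clears the Map's Spawned flag.
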(event Custom|OnBombCreated_Event
  (params (Bomb :type Bomb%20Object%20Reference))
  (Variables|Default|SetBombs (+ (Variables|Default|GetBombs) 1)))

(event Custom|OnBombDestroyed_Event
  (params (Bomb :type Bomb%20Object%20Reference))
  (Variables|Default|SetBombs (- (Variables|Default|GetBombs) 1)))

(event Custom|OnBombermanCreated_Event
  (params (Bomberman :type Bomberman%20Character%20Object%20Reference))
  (bind _asgod_player_controller (Utilities|Casting|CastToGodPlayerController (Game|GetPlayerController 0))
    (:then
      (bind _returnvalue (AI|GetAIController Bomberman))
      (bind _asbomber_man_aicontroller (Utilities|Casting|CastToBomberManAIController _returnvalue)
        (:then
          (Default|SetAIController _asgod_player_controller _asbomber_man_aicontroller)
          (Variables|/Game/Blueprints/BomberManAIController.BomberManAIController_C|SetMap _asbomber_man_aicontroller (Variables|Default|GetMap)))
        (:CastFailed
          (Rendering|Debug|DrawDebugString "0, 0, 0" "\"Whoops" 0 "(R=1.000000,G=1.000000,B=1.000000,A=1.000000)"))))
    (:CastFailed
      (Rendering|Debug|DrawDebugString "0, 0, 0" "\"Whoops" 0 "(R=1.000000,G=1.000000,B=1.000000,A=1.000000)"))))

(event Custom|OnBombermanDestroyed_Event
  (params (Bomberman :type Bomberman%20Character%20Object%20Reference))
  (Variables|/Game/Blueprints/Level/Map.Map_C|SetSpawned (Variables|Default|GetMap) false))

(event EventBeginPlay)

(event EventTick
  (params (DeltaSeconds :type Float%20%28single-precision%29)))

(fn ConstructionScript)