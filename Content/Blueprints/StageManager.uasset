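; Stage manager for the Bomberman game that steps through an ordered list of stages as streamed levels.
; It registers itself on the game instance and loads the current stage on BeginPlay.
; LevelFinished advances the index, then swaps streaming levels via load and visibility flags, or changes game instance state after the last stage.
; LevelLoaded destroys all Bomberman characters and clears the game mode map's Spawned flag.
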(event Custom|LevelFinished
  (Variables|Default|SetPrevStageIndex (Variables|Default|GetStageIndex))
  (Variables|Default|SetStageIndex (+ (Variables|Default|GetStageIndex) 1))
  (if (== (Variables|Default|GetStageIndex) (Utilities|Array|Length (Variables|Default|GetStages)))
    (bind _asbomberman_game_instance (Utilities|Casting|CastToBombermanGameInstance (Game|GetGameInstance)))
    (Default|SetState _asbomberman_game_instance "NewEnumerator7")
    (else
      (CallFunction|LoadLevel))))

(event Custom|LevelLoaded
  (bind _outactors (Actor|GetAllActorsOfClass "/Game/Blueprints/BombermanCharacter.BombermanCharacter_C"))
  (for _array_element _outactors
    (Actor|DestroyActor _array_element))
  (bind _asbomber_man_game (Utilities|Casting|CastToBomberManGame (Game|GetGameMode)))
  (Variables|/Game/Blueprints/Level/Map.Map_C|SetSpawned (Variables|/Game/Blueprints/BomberManGame.BomberManGame_C|GetMap _asbomber_man_game) false))

(event EventBeginPlay
  (bind _asbomberman_game_instance (Utilities|Casting|CastToBombermanGameInstance (Game|GetGameInstance)))
  (bind _output_get (Variables|/Game/Blueprints/BombermanGameInstance.BombermanGameInstance_C|SetStageManager _asbomberman_game_instance self))
  (CallFunction|LoadLevel _output_get))

(event EventActorBeginOverlap
  (params (OtherActor :type Actor%20Object%20Reference)))

(event EventTick
  (params (DeltaSeconds :type Float%20%28single-precision%29)))

(fn ConstructionScript
  (bind _asbomberman_game_instance (Utilities|Casting|CastToBombermanGameInstance (Game|GetGameInstance)))
  (Variables|/Game/Blueprints/BombermanGameInstance.BombermanGameInstance_C|SetStageManager _asbomberman_game_instance self))

(fn LoadLevel
  (bind _stages (Variables|Default|GetStages))
  (bind _prevstageindex (Variables|Default|GetPrevStageIndex))
  (bind _stages_2 (Variables|Default|GetStages))
  (bind _stageindex (Variables|Default|GetStageIndex))
  (bind _item (Utilities|Array|Get(acopy) _stages_2 _stageindex))
  (bind _item_2 (Utilities|Array|Get(acopy) _stages _prevstageindex))
  (bind _returnvalue (Class|GameplayStatics|GetStreamingLevel _item_2))
  (bind _returnvalue_2 (Class|GameplayStatics|GetStreamingLevel _item))
  (Variables|/Script/Engine.LevelStreaming|SetbShouldBeLoaded _returnvalue_2 true)
  (Variables|/Script/Engine.LevelStreaming|SetbShouldBeVisible _returnvalue_2 true)
  (Input|SetInputModeGameOnly (Game|GetPlayerController 0))
  (if (!= (Variables|Default|GetPrevStageIndex) -1)
    (Variables|/Script/Engine.LevelStreaming|SetbShouldBeLoaded _returnvalue false)
    (Variables|/Script/Engine.LevelStreaming|SetbShouldBeVisible _returnvalue false)))