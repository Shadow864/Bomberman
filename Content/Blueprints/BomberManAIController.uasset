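; AI controller for the Bomberman pawn that turns four directional action events into fixed-distance, grid-like steps along world X and Y.
; Each event sets a direction and, only while no move is in progress, calculates a goal from the pawn's location.
; CalculateGoal spawns a DebugSphere at that goal, and MoveTo pathfinds there with navmesh projection.
; The IsValid bounds helper is never called and never sets a true result.
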(event Custom|ActionLeft
  (Variables|Default|SetMovementDirection "-1.000000, 0, 0")
  (bind _ismoving (CallFunction|IsMoving))
  (if (not _ismoving)
    (bind _output_get (Variables|Default|SetMovementGoal (CallFunction|CalculateGoal (Variables|Default|GetMovementDirection) (Variables|Default|GetMovementDistance))))
    (CallFunction|Moveto _output_get)))

(event Custom|Action%20Right
  (Variables|Default|SetMovementDirection "1.000000, 0, 0")
  (bind _ismoving (CallFunction|IsMoving))
  (if (not _ismoving)
    (bind _output_get (Variables|Default|SetMovementGoal (CallFunction|CalculateGoal (Variables|Default|GetMovementDirection) (Variables|Default|GetMovementDistance))))
    (CallFunction|Moveto _output_get)))

(event Custom|Action%20Up
  (Variables|Default|SetMovementDirection "0.000000,-1.000000, 0")
  (bind _ismoving (CallFunction|IsMoving))
  (if (not _ismoving)
    (bind _output_get (Variables|Default|SetMovementGoal (CallFunction|CalculateGoal (Variables|Default|GetMovementDirection) (Variables|Default|GetMovementDistance))))
    (CallFunction|Moveto _output_get)))

(event Custom|Action%20Down
  (Variables|Default|SetMovementDirection "0.000000,1.000000,0.000000")
  (bind _ismoving (CallFunction|IsMoving))
  (if (not _ismoving)
    (bind _output_get (Variables|Default|SetMovementGoal (CallFunction|CalculateGoal (Variables|Default|GetMovementDirection) (Variables|Default|GetMovementDistance))))
    (CallFunction|Moveto _output_get)))

(event EventBeginPlay)

(fn ConstructionScript)

(fn IsMoving
  (return (not (Utilities|Enum|Equal(Enum) (Class|AIController|GetMoveStatus) "Idle"))))

(fn CalculateGoal
  (params (Direction :type Vector) (Distance :type Float%20%28single-precision%29))
  (bind _returnvalue (* Direction Distance))
  (bind _returnvalue_2 (Pawn|GetControlledPawn))
  (bind _returnvalue_3 (Transformation|GetActorLocation _returnvalue_2))
  (bind _returnvalue_4 (+ _returnvalue _returnvalue_3))
  (Game|SpawnActorfromClass "/Game/Blueprints/DebugSphere.DebugSphere_C" (Math|Transform|MakeTransform _returnvalue_4) "Undefined" 0 0)
  (return _returnvalue_4))

(fn Moveto
  (params (Goal :type Vector))
  (AI|Navigation|MovetoLocation Goal 1.0 false true true true 0 false))

(fn IsValid
  (params (Point :type Vector) (Min :type Float%20%28single-precision%29) (Max :type Float%20%28single-precision%29))
  (bind (_x _y) (Math|Vector|BreakVector Point))
  (if (> _x Max)
    (LocalVariables|SetResult false :!label _label)
    (elif (< _x Min)
      (goto _label)
      (elif (> _y Max)
        (goto _label)
        (elif (< _y Min)
          (goto _label)
          (else
            _)))))
  (return (LocalVariables|GetResult)))