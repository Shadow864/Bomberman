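; Base logic for a Bomberman enemy that dies in explosions and awards score.
; BeginPlay caches the BombermanGameInstance, and a capsule overlap with an explosion effect sets IsDead once, then adds its Points to the score at the enemy's location.
; Destruction is deferred to AnimDeathEnd, which nothing in this graph calls.
; GetPoints exposes the score value, while leftover behavior tree and destroy nodes are unconnected.
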(event OnComponentBeginOverlap(CapsuleComponent)
  (params (OtherActor :type Actor%20Object%20Reference) (OtherComp :type Primitive%20Component%20Object%20Reference) (OtherBodyIndex :type Integer) (bFromSweep :type Boolean) (SweepResult :type Hit%20Result%20Structure%20%28by%20ref%29))
  (Utilities|Casting|CastToBlueprint_Effect_Explosion OtherActor)
  (if (not (Variables|Default|GetIsDead))
    (Variables|Default|SetIsDead true)
    (Default|AddScore (Variables|Default|GetGameInstance) (Variables|Default|GetPoints) (Transformation|GetActorLocation))))

(event EventBeginPlay
  (bind _asbomberman_game_instance (Utilities|Casting|CastToBombermanGameInstance (Game|GetGameInstance)))
  (Variables|Default|SetGameInstance _asbomberman_game_instance))

(event EventActorBeginOverlap
  (params (OtherActor :type Actor%20Object%20Reference)))

(event EventTick
  (params (DeltaSeconds :type Float%20%28single-precision%29)))

(fn ConstructionScript)

(fn AnimDeathEnd
  (Actor|DestroyActor))

(fn GetPoints
  (return (Variables|Default|GetPoints)))