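; Behavior tree task that moves the controlled pawn to the TargetPosition blackboard vector.
; It runs AIMoveTo, then snaps the pawn onto the target on both success and failure, reporting the matching result.
; Tick aborts and stops movement when the stored destination differs from the current target with Z zeroed.
; GetDirectionVector is an uncalled stub returning zero for every direction.
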(event EventReceiveExecuteAI
  (params (OwnerController :type AI%20Controller%20Object%20Reference) (ControlledPawn :type Pawn%20Object%20Reference))
  (bind _output_get (Variables|Default|SetDestination (Class|BTFunctionLibrary|GetBlackboardValueasVector (Variables|Default|GetTargetPosition))))
  (AI|AIMoveTo OwnerController ControlledPawn _output_get 0 1.0 false
    (:OnSuccess
      (Transformation|SetActorLocation ControlledPawn _output_get false false)
      (AI|BehaviorTree|FinishExecute true))
    (:OnFail
      (Transformation|SetActorLocation ControlledPawn (Class|BTFunctionLibrary|GetBlackboardValueasVector (Variables|Default|GetTargetPosition)) false false)
      (AI|BehaviorTree|FinishExecute false))))

(event EventReceiveTickAI
  (params (OwnerController :type AI%20Controller%20Object%20Reference) (ControlledPawn :type Pawn%20Object%20Reference) (DeltaSeconds :type Float%20%28single-precision%29))
  (bind _targetposition (Variables|Default|GetTargetPosition))
  (bind _returnvalue (Class|BTFunctionLibrary|GetBlackboardValueasVector _targetposition))
  (bind (_x _y) (Math|Vector|BreakVector _returnvalue))
  (if (Math|Vector|NotEqual(Vector) (Variables|Default|GetDestination) (Math|Vector|MakeVector _x _y 0.0) 0.0001)
    (Class|BTTaskBlueprintBase|FinishAbort)
    (AI|Navigation|StopMovement OwnerController)))

(event EventReceiveAbortAI
  (params (OwnerController :type AI%20Controller%20Object%20Reference) (ControlledPawn :type Pawn%20Object%20Reference))
  (AI|Navigation|StopMovement OwnerController)
  (AI|BehaviorTree|FinishExecute false))

(fn GetDirectionVector
  (params (Direction :type Direction%20Enum))
  (switch Utilities|FlowControl|Switch|SwitchonDirection Direction
    (:NewEnumerator0
      (return ""))
    (:NewEnumerator1
      (return ""))
    (:NewEnumerator2
      (return ""))
    (:NewEnumerator3
      (return ""))))