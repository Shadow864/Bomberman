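; Behavior tree service that picks an AI's next movement target on a 100-unit tile grid, despite its FindTarget name choosing directions at random.
; Each tick it probes the four neighboring tiles from the current TargetPosition and randomly selects an unblocked direction.
; A long trace that ignores Destroyable actors finds a hit, which is snapped to the grid.
; The old target becomes StartPosition and the snapped point becomes TargetPosition.
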(event EventReceiveTickAI
  (params (OwnerController :type AI%20Controller%20Object%20Reference) (ControlledPawn :type Pawn%20Object%20Reference) (DeltaSeconds :type Float%20%28single-precision%29))
  (bind _targetposition (Variables|Default|GetTargetPosition))
  (bind _returnvalue (Class|BTFunctionLibrary|GetBlackboardValueasVector _targetposition))
  (bind (_x _y _z) (Math|Vector|BreakVector _returnvalue))
  (bind _returnvalue_2 (Math|Vector|MakeVector _x _y 3e+01))
  (bind _outactors (Actor|GetAllActorsOfClass "/Game/Blueprints/Destroyables/Destroyable.Destroyable_C"))
  (bind _outhit (Collision|LineTraceByChannel _returnvalue_2 (+ _returnvalue_2 (CallFunction|GetRandomDirection _returnvalue_2)) "TraceTypeQuery1" false _outactors "None"))
  (bind _returnvalue_3 (CallFunction|FindValidTilePosition (Math|Vector|MakeVector (.X (Math|Vector|BreakVector (.Location (Collision|BreakHitResult _outhit)))) (.Y (Math|Vector|BreakVector (.Location (Collision|BreakHitResult _outhit)))) _z) (Class|BTFunctionLibrary|GetBlackboardValueasVector (Variables|Default|GetTargetPosition))))
  (AI|BehaviorTree|SetBlackboardValueasVector (Variables|Default|GetStartPosition) (Class|BTFunctionLibrary|GetBlackboardValueasVector (Variables|Default|GetTargetPosition)))
  (AI|BehaviorTree|SetBlackboardValueasVector (Variables|Default|GetTargetPosition) _returnvalue_3))

(fn GetRandomDirection
  (params (Position :type Vector))
  (bind _directions (CallFunction|GetAvaiableDirections Position))
  (Rendering|Debug|DrawDebugString "0, 0, 0" (Utilities|String|EnumtoString (Utilities|Array|Get(acopy) _directions (Math|Random|RandomIntegerinRange 0 (- (Utilities|Array|Length _directions) 1)))) 0 "(R=1.000000,G=1.000000,B=1.000000,A=1.000000)" 1.0)
  (return (* (CallFunction|GetDirectionVector (Utilities|Array|Get(acopy) _directions (Math|Random|RandomIntegerinRange 0 (- (Utilities|Array|Length _directions) 1)))) 2e+03)))

(fn FindValidTilePosition
  (params (HitLocation :type Vector) (AILocation :type Vector))
  (bind _returnvalue (/ HitLocation "100.000000,100.000000,1.000000"))
  (bind (_x _y _z) (Math|Vector|BreakVector _returnvalue))
  (LocalVariables|SetLocaion AILocation)
  (LocalVariables|SetX _x)
  (LocalVariables|SetY _y)
  (LocalVariables|SetZ _z)
  (if (and (>= (Math|Float|%(Float) (LocalVariables|GetX) 1.0) 0.5) (> (.X (Math|Vector|BreakVector (/ (LocalVariables|GetLocaion) "100.000000,100.000000,1.000000"))) (LocalVariables|GetX)))
    (LocalVariables|SetX (+ (LocalVariables|GetX) 1.0)))
  (if (and (>= (Math|Float|%(Float) (LocalVariables|GetY) 1.0) 0.5) (> (.Y (Math|Vector|BreakVector (/ (LocalVariables|GetLocaion) "100.000000,100.000000,1.000000"))) (LocalVariables|GetY)))
    (LocalVariables|SetY (+ (LocalVariables|GetY) 1.0)))
  (return (Math|Vector|MakeVector (* 100 (Math|Conversions|ToFloat(Integer) (Math|Float|Truncate (LocalVariables|GetX)))) (* 100 (Math|Conversions|ToFloat(Integer) (Math|Float|Truncate (LocalVariables|GetY)))) 0.0)))

(fn GetDirectionVector
  (params (Direction :type Direction%20Enum))
  (switch Utilities|FlowControl|Switch|SwitchonDirection Direction
    (:NewEnumerator0
      (return "1.000000,0,0"))
    (:NewEnumerator1
      (return "-1.000000,0,0"))
    (:NewEnumerator2
      (return "0,-1.000000,0"))
    (:NewEnumerator3
      (return "0,1.000000,0"))))

(fn GetAvaiableDirections
  (params (Position :type Vector))
  (LocalVariables|SetStart%20Position Position)
  (bind _enumvalue (|ForEachDirection)
    (:LoopBody
      (bind _returnvalue (Collision|LineTraceByChannel (LocalVariables|GetStart%20Position) (+ (* (CallFunction|GetDirectionVector _enumvalue) 1e+02) (LocalVariables|GetStart%20Position)) "TraceTypeQuery1" true 0 "ForOneFrame"))
      (if (not _returnvalue)
        (Utilities|Array|Add (LocalVariables|GetDirs) _enumvalue)))
    (:then
      (return (LocalVariables|GetDirs)))))