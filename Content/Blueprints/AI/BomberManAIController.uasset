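; AI controller that drives a BombermanCharacter around a tile-based map through directional and fire action events.
; Each direction event shares one path that checks the next tile is empty and no move is underway, updates the grid position, then calls MoveToLocation toward that tile.
; IsMoving compares pawn location to the stored goal; firing spawns a bomb at the current tile.
; CalculateGoal and IsValid are helpers this graph never calls.
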(event Custom|ActionLeft
  (bind _map (Variables|Default|GetMap))
  (bind _tilesize (Variables|/Game/Blueprints/Level/Map.Map_C|GetTileSize _map))
  (bind (_width _height) (Utilities|Struct|BreakSize _tilesize))
  (Variables|Default|SetDirection (Utilities|Struct|MakePosition2D 0 -1))
  (Variables|Default|SetMovementDirection "0.000000,-1.000000, 0")
  (bind _asbomberman_character (Utilities|Casting|CastToBombermanCharacter (Pawn|GetControlledPawn)))
  (bind _result (Default|IsEmpty (Variables|Default|GetMap) (Utilities|Struct|MakePosition2D (+ (.X (Utilities|Struct|BreakPosition2D (Variables|/Game/Blueprints/Player/BombermanCharacter.BombermanCharacter_C|GetCurrentPosition _asbomberman_character))) (.X (Utilities|Struct|BreakPosition2D (Variables|Default|GetDirection)))) (+ (.Y (Utilities|Struct|BreakPosition2D (Variables|/Game/Blueprints/Player/BombermanCharacter.BombermanCharacter_C|GetCurrentPosition _asbomberman_character))) (.Y (Utilities|Struct|BreakPosition2D (Variables|Default|GetDirection)))))))
  (if _result
    (bind _ismoving (CallFunction|IsMoving))
    (if (not _ismoving)
      (bind _output_get (Variables|/Game/Blueprints/Player/BombermanCharacter.BombermanCharacter_C|SetCurrentPosition _asbomberman_character (Utilities|Struct|MakePosition2D (+ (.X (Utilities|Struct|BreakPosition2D (Variables|/Game/Blueprints/Player/BombermanCharacter.BombermanCharacter_C|GetCurrentPosition _asbomberman_character))) (.X (Utilities|Struct|BreakPosition2D (Variables|Default|GetDirection)))) (+ (.Y (Utilities|Struct|BreakPosition2D (Variables|/Game/Blueprints/Player/BombermanCharacter.BombermanCharacter_C|GetCurrentPosition _asbomberman_character))) (.Y (Utilities|Struct|BreakPosition2D (Variables|Default|GetDirection)))))))
      (bind _output_get_2 (Variables|Default|SetMovementGoal (Math|Vector|MakeVector (Math|Conversions|ToFloat(Integer) (* (.X (Utilities|Struct|BreakPosition2D _output_get)) _width)) (Math|Conversions|ToFloat(Integer) (* (.Y (Utilities|Struct|BreakPosition2D _output_get)) _height)) 9e+01)))
      (CallFunction|Moveto _output_get_2))))

(event Custom|Action%20Right
  (bind _map (Variables|Default|GetMap))
  (bind _tilesize (Variables|/Game/Blueprints/Level/Map.Map_C|GetTileSize _map))
  (bind (_width _height) (Utilities|Struct|BreakSize _tilesize))
  (Variables|Default|SetDirection (Utilities|Struct|MakePosition2D 0 1))
  (Variables|Default|SetMovementDirection "0.000000,1.000000,0.000000")
  (bind _asbomberman_character (Utilities|Casting|CastToBombermanCharacter (Pawn|GetControlledPawn)))
  (bind _result (Default|IsEmpty (Variables|Default|GetMap) (Utilities|Struct|MakePosition2D (+ (.X (Utilities|Struct|BreakPosition2D (Variables|/Game/Blueprints/Player/BombermanCharacter.BombermanCharacter_C|GetCurrentPosition _asbomberman_character))) (.X (Utilities|Struct|BreakPosition2D (Variables|Default|GetDirection)))) (+ (.Y (Utilities|Struct|BreakPosition2D (Variables|/Game/Blueprints/Player/BombermanCharacter.BombermanCharacter_C|GetCurrentPosition _asbomberman_character))) (.Y (Utilities|Struct|BreakPosition2D (Variables|Default|GetDirection)))))))
  (if _result
    (bind _ismoving (CallFunction|IsMoving))
    (if (not _ismoving)
      (bind _output_get (Variables|/Game/Blueprints/Player/BombermanCharacter.BombermanCharacter_C|SetCurrentPosition _asbomberman_character (Utilities|Struct|MakePosition2D (+ (.X (Utilities|Struct|BreakPosition2D (Variables|/Game/Blueprints/Player/BombermanCharacter.BombermanCharacter_C|GetCurrentPosition _asbomberman_character))) (.X (Utilities|Struct|BreakPosition2D (Variables|Default|GetDirection)))) (+ (.Y (Utilities|Struct|BreakPosition2D (Variables|/Game/Blueprints/Player/BombermanCharacter.BombermanCharacter_C|GetCurrentPosition _asbomberman_character))) (.Y (Utilities|Struct|BreakPosition2D (Variables|Default|GetDirection)))))))
      (bind _output_get_2 (Variables|Default|SetMovementGoal (Math|Vector|MakeVector (Math|Conversions|ToFloat(Integer) (* (.X (Utilities|Struct|BreakPosition2D _output_get)) _width)) (Math|Conversions|ToFloat(Integer) (* (.Y (Utilities|Struct|BreakPosition2D _output_get)) _height)) 9e+01)))
      (CallFunction|Moveto _output_get_2))))

(event Custom|Action%20Up
  (bind _map (Variables|Default|GetMap))
  (bind _tilesize (Variables|/Game/Blueprints/Level/Map.Map_C|GetTileSize _map))
  (bind (_width _height) (Utilities|Struct|BreakSize _tilesize))
  (Variables|Default|SetDirection (Utilities|Struct|MakePosition2D 1))
  (Variables|Default|SetMovementDirection "0.000000,-1.000000, 0")
  (bind _asbomberman_character (Utilities|Casting|CastToBombermanCharacter (Pawn|GetControlledPawn)))
  (bind _result (Default|IsEmpty (Variables|Default|GetMap) (Utilities|Struct|MakePosition2D (+ (.X (Utilities|Struct|BreakPosition2D (Variables|/Game/Blueprints/Player/BombermanCharacter.BombermanCharacter_C|GetCurrentPosition _asbomberman_character))) (.X (Utilities|Struct|BreakPosition2D (Variables|Default|GetDirection)))) (+ (.Y (Utilities|Struct|BreakPosition2D (Variables|/Game/Blueprints/Player/BombermanCharacter.BombermanCharacter_C|GetCurrentPosition _asbomberman_character))) (.Y (Utilities|Struct|BreakPosition2D (Variables|Default|GetDirection)))))))
  (if _result
    (bind _ismoving (CallFunction|IsMoving))
    (if (not _ismoving)
      (bind _output_get (Variables|/Game/Blueprints/Player/BombermanCharacter.BombermanCharacter_C|SetCurrentPosition _asbomberman_character (Utilities|Struct|MakePosition2D (+ (.X (Utilities|Struct|BreakPosition2D (Variables|/Game/Blueprints/Player/BombermanCharacter.BombermanCharacter_C|GetCurrentPosition _asbomberman_character))) (.X (Utilities|Struct|BreakPosition2D (Variables|Default|GetDirection)))) (+ (.Y (Utilities|Struct|BreakPosition2D (Variables|/Game/Blueprints/Player/BombermanCharacter.BombermanCharacter_C|GetCurrentPosition _asbomberman_character))) (.Y (Utilities|Struct|BreakPosition2D (Variables|Default|GetDirection)))))))
      (bind _output_get_2 (Variables|Default|SetMovementGoal (Math|Vector|MakeVector (Math|Conversions|ToFloat(Integer) (* (.X (Utilities|Struct|BreakPosition2D _output_get)) _width)) (Math|Conversions|ToFloat(Integer) (* (.Y (Utilities|Struct|BreakPosition2D _output_get)) _height)) 9e+01)))
      (CallFunction|Moveto _output_get_2))))

(event Custom|Action%20Down
  (bind _map (Variables|Default|GetMap))
  (bind _tilesize (Variables|/Game/Blueprints/Level/Map.Map_C|GetTileSize _map))
  (bind (_width _height) (Utilities|Struct|BreakSize _tilesize))
  (Variables|Default|SetDirection (Utilities|Struct|MakePosition2D -1))
  (Variables|Default|SetMovementDirection "0.000000,1.000000,0.000000")
  (bind _asbomberman_character (Utilities|Casting|CastToBombermanCharacter (Pawn|GetControlledPawn)))
  (bind _result (Default|IsEmpty (Variables|Default|GetMap) (Utilities|Struct|MakePosition2D (+ (.X (Utilities|Struct|BreakPosition2D (Variables|/Game/Blueprints/Player/BombermanCharacter.BombermanCharacter_C|GetCurrentPosition _asbomberman_character))) (.X (Utilities|Struct|BreakPosition2D (Variables|Default|GetDirection)))) (+ (.Y (Utilities|Struct|BreakPosition2D (Variables|/Game/Blueprints/Player/BombermanCharacter.BombermanCharacter_C|GetCurrentPosition _asbomberman_character))) (.Y (Utilities|Struct|BreakPosition2D (Variables|Default|GetDirection)))))))
  (if _result
    (bind _ismoving (CallFunction|IsMoving))
    (if (not _ismoving)
      (bind _output_get (Variables|/Game/Blueprints/Player/BombermanCharacter.BombermanCharacter_C|SetCurrentPosition _asbomberman_character (Utilities|Struct|MakePosition2D (+ (.X (Utilities|Struct|BreakPosition2D (Variables|/Game/Blueprints/Player/BombermanCharacter.BombermanCharacter_C|GetCurrentPosition _asbomberman_character))) (.X (Utilities|Struct|BreakPosition2D (Variables|Default|GetDirection)))) (+ (.Y (Utilities|Struct|BreakPosition2D (Variables|/Game/Blueprints/Player/BombermanCharacter.BombermanCharacter_C|GetCurrentPosition _asbomberman_character))) (.Y (Utilities|Struct|BreakPosition2D (Variables|Default|GetDirection)))))))
      (bind _output_get_2 (Variables|Default|SetMovementGoal (Math|Vector|MakeVector (Math|Conversions|ToFloat(Integer) (* (.X (Utilities|Struct|BreakPosition2D _output_get)) _width)) (Math|Conversions|ToFloat(Integer) (* (.Y (Utilities|Struct|BreakPosition2D _output_get)) _height)) 9e+01)))
      (CallFunction|Moveto _output_get_2))))

(event Custom|Action%20Fire
  (bind _asbomberman_character (Utilities|Casting|CastToBombermanCharacter (Pawn|GetControlledPawn)))
  (Default|SpawnBomb (Variables|Default|GetMap) (Variables|/Game/Blueprints/Player/BombermanCharacter.BombermanCharacter_C|GetCurrentPosition _asbomberman_character)))

(event EventBeginPlay)

(fn ConstructionScript)

(fn IsMoving
  (bind _movementgoal (Variables|Default|GetMovementGoal))
  (return (not (or (Math|Vector|Equal(Vector) _movementgoal "0, 0, 0" 1.0) (Math|Vector|Equal(Vector) (Transformation|GetActorLocation (Pawn|GetControlledPawn)) _movementgoal 1e+01)))))

(fn CalculateGoal
  (params (Direction :type Vector) (Distance :type Float%20%28single-precision%29))
  (bind _returnvalue (* Direction Distance))
  (bind _returnvalue_2 (Pawn|GetControlledPawn))
  (bind _returnvalue_3 (Transformation|GetActorLocation _returnvalue_2))
  (bind _returnvalue_4 (+ _returnvalue _returnvalue_3))
  (Game|SpawnActorfromClass "/Game/Blueprints/DebugSphere.DebugSphere_C" (Math|Transform|MakeTransform _returnvalue_4) "Undefined" 0 0)
  (return _returnvalue_4))

(fn Moveto
  (params (Goal :type Vector))
  (AI|Navigation|MovetoLocation Goal 1.0 false true false false 0 false))

(fn IsValid
  (params (Point :type Vector) (Min :type Float%20%28single-precision%29) (Max :type Float%20%28single-precision%29))
  (bind (_x _y) (Math|Vector|BreakVector Point))
  (if (> _x Max)
    (LocalVariables|SetResult false :!label _label)
    (elif (< _x Min)
      (goto _label)
      (elif (> _y Max)
        (goto _label)
        (elif (< _y Min)
          (goto _label)
          (else
            _)))))
  (return (LocalVariables|GetResult)))