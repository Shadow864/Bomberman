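; Behavior tree service that stops an AI pawn's target position from lying past an obstacle on a tile grid.
; Each tick it runs a short, low visibility trace from the pawn toward the TargetPosition blackboard value.
; On a hit, FindValidTilePosition snaps the impact to 100-unit grid coordinates, biased toward the pawn's side, and overwrites TargetPosition.
; A GetRandomDirection helper returns one of four axis-aligned offsets but is not called here.
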(event EventReceiveTickAI
  (params (OwnerController :type AI%20Controller%20Object%20Reference) (ControlledPawn :type Pawn%20Object%20Reference) (DeltaSeconds :type Float%20%28single-precision%29))
  (bind _returnvalue (Transformation|GetActorLocation ControlledPawn))
  (bind (_x _y _z) (Math|Vector|BreakVector _returnvalue))
  (bind _returnvalue_2 (Math|Vector|MakeVector _x _y 4e+01))
  (bind (_outhit _returnvalue_3) (Collision|LineTraceByChannel _returnvalue_2 (+ (* (Math|Vector|Normalize (- (Class|BTFunctionLibrary|GetBlackboardValueasVector (Variables|Default|GetTargetPosition)) _returnvalue)) "55.000000,55.000000, 0") _returnvalue_2) "TraceTypeQuery1" false 0 "None"))
  (if _returnvalue_3
    (AI|GetAIController ControlledPawn)
    (bind _returnvalue_4 (CallFunction|FindValidTilePosition (Math|Vector|MakeVector (.X (Math|Vector|BreakVector (.Location (Collision|BreakHitResult _outhit)))) (.Y (Math|Vector|BreakVector (.Location (Collision|BreakHitResult _outhit)))) _z) _returnvalue))
    (AI|BehaviorTree|SetBlackboardValueasVector (Variables|Default|GetTargetPosition) _returnvalue_4)))

(fn GetRandomDirection
  (switch Utilities|FlowControl|Switch|SwitchonDirection (Utilities|Enum|ByteToEnumDirection (Math|Conversions|ToByte(Integer) (Math|Random|RandomIntegerinRange 0 3)))
    (:NewEnumerator0
      (return "2000.000000,0,0"))
    (:NewEnumerator1
      (return "-2000.000000,0,0"))
    (:NewEnumerator2
      (return "0,-2000.000000,0"))
    (:NewEnumerator3
      (return "0,2000.000000,0"))))

(fn FindValidTilePosition
  (params (HitLocation :type Vector) (AILocation :type Vector))
  (bind _output_get (LocalVariables|SetLocalHitLocation HitLocation))
  (LocalVariables|SetLocaion AILocation)
  (LocalVariables|SetX (.X (Math|Vector|BreakVector (/ _output_get "100.000000,100.000000,1.000000"))))
  (LocalVariables|SetY (.Y (Math|Vector|BreakVector (/ _output_get "100.000000,100.000000,1.000000"))))
  (LocalVariables|SetZ (.Z (Math|Vector|BreakVector (/ _output_get "100.000000,100.000000,1.000000"))))
  (if (and (>= (Math|Float|%(Float) (LocalVariables|GetX) 1.0) 0.4) (> (.X (Math|Vector|BreakVector (/ (LocalVariables|GetLocaion) "100.000000,100.000000,1.000000"))) (LocalVariables|GetX)))
    (LocalVariables|SetX (+ (LocalVariables|GetX) 1.0)))
  (if (and (>= (Math|Float|%(Float) (LocalVariables|GetY) 1.0) 0.4) (> (.Y (Math|Vector|BreakVector (/ (LocalVariables|GetLocaion) "100.000000,100.000000,1.000000"))) (LocalVariables|GetY)))
    (LocalVariables|SetY (+ (LocalVariables|GetY) 1.0)))
  (return (Math|Vector|MakeVector (* 100 (Math|Conversions|ToFloat(Integer) (Math|Float|Truncate (LocalVariables|GetX)))) (* 100 (Math|Conversions|ToFloat(Integer) (Math|Float|Truncate (LocalVariables|GetY)))) (.Z (Math|Vector|BreakVector (LocalVariables|GetLocaion))))))