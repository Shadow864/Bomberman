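; Game instance for a Bomberman game that drives the game state machine and holds score and power-up counts across level loads.
; SetState ignores repeated states; each change broadcasts StateChanged and triggers menu music, level loading, or resets on unload and restart.
; Power-ups live in an array indexed by enum type, seeded with per-type defaults.
; AddScore also spawns a FloatingScore actor, and level queries read from StageManager.
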(event Custom|StateChanged_Event
  (params (Prev :type State%20Enum) (NewParam :type State%20Enum))
  (Default|CallStateChanged NewParam Prev)
  (switch Utilities|FlowControl|Switch|SwitchonState NewParam
    (:NewEnumerator0
      (CallFunction|SetState "NewEnumerator1"))
    (:NewEnumerator1
      (Audio|PlaySound2D "/Game/Audio/02-title.02-title" 1.0 1.0 1.0))
    (:NewEnumerator2
      (Game|OpenLevel(byName) "WorldLevel"))
    (:NewEnumerator6
      (Variables|Default|SetScore 0)
      (Game|OpenLevel(byName) "MainMenuLevel"))
    (:NewEnumerator8
      (Variables|Default|SetScore 0)
      (CallFunction|InitPowerUps)
      (CallFunction|SetState "NewEnumerator2"))))

(event EventInit
  (CallFunction|InitPowerUps))

(fn SetState
  (params (State :type State%20Enum))
  (if (Utilities|Enum|NotEqual(Enum) State (Variables|Default|GetGameState))
    (LocalVariables|SetPrevState (Variables|Default|GetGameState))
    (Variables|Default|SetGameState State)
    (CallFunction|StateChangedEvent (LocalVariables|GetPrevState) (Variables|Default|GetGameState))))

(fn InitPowerUps
  (Utilities|Array|Resize (Variables|Default|GetPowerUps) (Math|Conversions|ToInteger(Byte) (- (Utilities|Enum|LiteralenumPowerUpType "NewEnumerator4") 1)))
  (bind _enumvalue (|ForEachPowerUpType)
    (:LoopBody
      (bind _count (CallFunction|GetInitialPowerUpCount _enumvalue))
      (Utilities|Array|SetArrayElem (Variables|Default|GetPowerUps) (Math|Conversions|ToInteger(Byte) _enumvalue) _count))))

(fn GetInitialPowerUpCount
  (params (Type :type PowerUpType%20Enum))
  (switch Utilities|FlowControl|Switch|SwitchonPowerUpType Type
    (:NewEnumerator0
      (return 0))
    (:NewEnumerator1
      (return 0))
    (:NewEnumerator2
      (return 1))
    (:NewEnumerator3
      (return 0))
    (:NewEnumerator4
      (return 0))))

(fn AddPowerUp
  (params (Type :type PowerUpType%20Enum))
  (bind _output_get (LocalVariables|SetIndex (Math|Conversions|ToInteger(Byte) Type)))
  (Utilities|Array|SetArrayElem (Variables|Default|GetPowerUps) _output_get (+ (Utilities|Array|Get(acopy) (Variables|Default|GetPowerUps) (LocalVariables|GetIndex)) 1)))

(fn GetPowerUpCount
  (params (Type :type PowerUpType%20Enum))
  (return (Utilities|Array|Get(acopy) (Variables|Default|GetPowerUps) (Math|Conversions|ToInteger(Byte) Type))))

(fn AddScore
  (params (Score :type Integer) (Position :type Vector))
  (if (> Score 0)
    (Game|SpawnActorfromClass "/Game/Blueprints/Score/FloatingScore.FloatingScore_C" (Math|Conversions|ToTransform(Vector) Position) "AlwaysSpawn" 0 Score 0)
    (Variables|Default|SetScore (+ Score (Variables|Default|GetScore)))))

(fn GetLevelIndex
  (return (Variables|/Game/Blueprints/StageManager.StageManager_C|GetStageIndex (Variables|Default|GetStageManager))))

(fn GetLevelName
  (return (Utilities|Array|Get(acopy) (Variables|/Game/Blueprints/StageManager.StageManager_C|GetStages (Variables|Default|GetStageManager)) (CallFunction|GetLevelIndex))))