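; PowerUp is a spinning pickup actor for a Bomberman-style game, removed when collected or blown up.
; Tick yaws the static mesh at a frame-rate-independent speed, and overlap with a BombermanCharacter or an explosion effect destroys the actor.
; GetPowerUpType reports a fixed enum type, while the overlap logic itself applies no effect to the character.
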(event EventBeginPlay)

(event EventActorBeginOverlap
  (params (OtherActor :type Actor%20Object%20Reference))
  (Utilities|Casting|CastToBombermanCharacter OtherActor
    (:then
      _)
    (:CastFailed
      (Utilities|Casting|CastToBlueprint_Effect_Explosion OtherActor)))
  (Actor|DestroyActor))

(event EventTick
  (params (DeltaSeconds :type Float%20%28single-precision%29))
  (Transformation|AddRelativeRotation (Variables|Default|GetStaticMesh) (Math|Rotator|MakeRotator 0.0 0.0 (* DeltaSeconds (Variables|Default|GetRatotionSpeed))) false false))

(fn ConstructionScript)

(fn GetPowerUpType
  (return "NewEnumerator0"))