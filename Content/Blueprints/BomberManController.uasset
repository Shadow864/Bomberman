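; BomberManController is a keyboard input controller that drives a BomberMan AI controller with the arrow keys.
; Every tick it polls the four arrow keys independently and calls the matching Up, Down, Left or Right action on the stored AiController.
; That reference is supplied externally through SetAIController and is used without a validity check.
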(event EventTick
  (params (DeltaSeconds :type Float%20%28single-precision%29))
  (Utilities|FlowControl|Sequence
    (:then_0
      (if (Game|Player|IsInputKeyDown "Up")
        (Default|ActionUp (Variables|Default|GetAiController))))
    (:then_1
      (if (Game|Player|IsInputKeyDown "Down")
        (Default|ActionDown (Variables|Default|GetAiController))))
    (:then_2
      (if (Game|Player|IsInputKeyDown "Left")
        (Default|ActionLeft (Variables|Default|GetAiController))))
    (:then_3
      (if (Game|Player|IsInputKeyDown "Right")
        (Default|ActionRight (Variables|Default|GetAiController))))))

(fn ConstructionScript)

(fn SetAIController
  (params (AiController :type Bomber%20Man%20AI%20Controller%20Object%20Reference))
  (Variables|Default|SetAiController AiController))