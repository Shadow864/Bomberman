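; Bomberman HUD Blueprint that shows the UI widget for each game state.
; On BeginPlay it binds to the BombermanGameInstance's state-changed event.
; Each change to Main Menu, Game, Pause or Summary creates a new widget, adds it to the viewport, and sets cursor visibility and input mode to UI-only for menus or game-only for play.
; It never removes earlier widgets itself.
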(event Custom|GameStateChanged
  (params (NewState :type State%20Enum) (PrevState :type State%20Enum))
  (bind _returnvalue (Game|GetPlayerController 0))
  (bind _returnvalue_2 (Game|GetPlayerController 0))
  (bind _returnvalue_3 (Game|GetPlayerController 0))
  (bind _returnvalue_4 (Game|GetPlayerController 0))
  (switch Utilities|FlowControl|Switch|SwitchonState NewState
    (:NewEnumerator1
      (bind _returnvalue_5 (UserInterface|CreateWidget "/Game/Menu/MainMenu.MainMenu_C"))
      (bind _output_get (Variables|Default|SetMainMenu _returnvalue_5))
      (UserInterface|Viewport|AddtoViewport _output_get 0)
      (Variables|/Script/Engine.PlayerController|SetbShowMouseCursor _returnvalue_2 true)
      (Input|SetInputModeUIOnly _returnvalue_2 (Variables|Default|GetMainMenu) true))
    (:NewEnumerator3
      (bind _returnvalue_6 (UserInterface|CreateWidget "/Game/HUD/HUD.HUD_C"))
      (bind _output_get_2 (Variables|Default|SetHUD _returnvalue_6))
      (UserInterface|Viewport|AddtoViewport _output_get_2 0)
      (Variables|/Script/Engine.PlayerController|SetbShowMouseCursor _returnvalue_4 false)
      (Input|SetInputModeGameOnly _returnvalue_4))
    (:NewEnumerator4
      (bind _returnvalue_7 (UserInterface|CreateWidget "/Game/Menu/PauseMenu.PauseMenu_C"))
      (bind _output_get_3 (Variables|Default|SetPause%20Menu _returnvalue_7))
      (UserInterface|Viewport|AddtoViewport _output_get_3 0)
      (Variables|/Script/Engine.PlayerController|SetbShowMouseCursor _returnvalue true)
      (Input|SetInputModeUIOnly _returnvalue (Variables|Default|GetPause%20Menu) true))
    (:NewEnumerator7
      (bind _returnvalue_8 (UserInterface|CreateWidget "/Game/Menu/SummaryMenu.SummaryMenu_C"))
      (bind _output_get_4 (Variables|Default|SetSummaryMenu _returnvalue_8))
      (UserInterface|Viewport|AddtoViewport _output_get_4 0)
      (Variables|/Script/Engine.PlayerController|SetbShowMouseCursor _returnvalue_3 true)
      (Input|SetInputModeUIOnly _returnvalue_3 (Variables|Default|GetSummaryMenu) true))))

(event EventBeginPlay
  (bind _asbomberman_game_instance (Utilities|Casting|CastToBombermanGameInstance (Game|GetGameInstance)))
  (EventDispatchers|AssignStateChanged _asbomberman_game_instance (delegate Custom|GameStateChanged)))

(event EventActorBeginOverlap
  (params (OtherActor :type Actor%20Object%20Reference)))

(event EventTick
  (params (DeltaSeconds :type Float%20%28single-precision%29)))

(fn ConstructionScript)