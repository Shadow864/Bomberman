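; Destroyable is a Bomberman level object that is destroyed on overlap, awarding points and optionally revealing a power-up or the level exit.
; The first overlap on its static mesh sets a Destroyed guard, then adds score at its location through the cached BombermanGameInstance.
; GetSpawnClassId maps the SpawnObject enum to a class, which spawns at the actor's transform before the actor destroys itself.
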(event OnComponentBeginOverlap(StaticMesh)
  (params (OtherActor :type Actor%20Object%20Reference) (OtherComp :type Primitive%20Component%20Object%20Reference) (OtherBodyIndex :type Integer) (bFromSweep :type Boolean) (SweepResult :type Hit%20Result%20Structure%20%28by%20ref%29))
  (if (not (Variables|Default|GetDestroyed))
    (Variables|Default|SetDestroyed true)
    (Default|AddScore (Variables|Default|GetGame%20Instance) (Variables|Default|GetPoints) (Transformation|GetActorLocation))
    (Game|SpawnActorfromClass (CallFunction|GetSpawnClassId (Variables|Default|GetSpawnObject)) (Transformation|GetActorTransform) "AlwaysSpawn" 0 0)
    (Actor|DestroyActor)))

(event EventBeginPlay
  (bind _asbomberman_game_instance (Utilities|Casting|CastToBombermanGameInstance (Game|GetGameInstance)))
  (Variables|Default|SetGame%20Instance _asbomberman_game_instance))

(event EventActorBeginOverlap
  (params (OtherActor :type Actor%20Object%20Reference)))

(event EventTick
  (params (DeltaSeconds :type Float%20%28single-precision%29)))

(fn ConstructionScript)

(fn GetSpawnClassId
  (params (Type :type SpawnType%20Enum))
  (switch Utilities|FlowControl|Switch|SwitchonSpawnType (Variables|Default|GetSpawnObject)
    (:NewEnumerator0
      (return 0))
    (:NewEnumerator1
      (return "/Game/Blueprints/PowerUps/PowerUp_Accelerator.PowerUp_Accelerator_C"))
    (:NewEnumerator2
      (return "/Game/Blueprints/PowerUps/PowerUpExplosionExpander.PowerUpExplosionExpander_C"))
    (:NewEnumerator3
      (return "/Game/Blueprints/PowerUps/PowerUpExtraBomb.PowerUpExtraBomb_C"))
    (:NewEnumerator4
      (return "/Game/Blueprints/PowerUps/PowerUpRemote.PowerUpRemote_C"))
    (:NewEnumerator5
      (return "/Game/Blueprints/Level/Exit.Exit_C"))))

(fn GetPoints
  (return (Variables|Default|GetPoints)))