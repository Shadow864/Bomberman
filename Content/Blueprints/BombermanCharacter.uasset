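; Bomberman character Blueprint that handles being hit by explosions and picking up power-ups.
; It reports its creation and destruction to the BomberManGame game mode.
; Overlapping an explosion effect applies damage to itself, while actors implementing PowerUpInterface pass their power-up type to the game instance.
; Any damage is fatal: it sets a new state on the game instance and destroys the character.
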(event Game|Damage|EventAnyDamage
  (params (Damage :type Float%20%28single-precision%29) (DamageType :type Damage%20Type%20Object%20Reference) (InstigatedBy :type Controller%20Object%20Reference) (DamageCauser :type Actor%20Object%20Reference))
  (bind _asbomberman_game_instance (Utilities|Casting|CastToBombermanGameInstance (Game|GetGameInstance)))
  (Default|SetState _asbomberman_game_instance "NewEnumerator7")
  (Actor|DestroyActor))

(event EventDestroyed
  (bind _asbomber_man_game (Utilities|Casting|CastToBomberManGame (Game|GetGameMode)))
  (Default|OnBombermanDestroyedEvent _asbomber_man_game self))

(event EventBeginPlay
  (bind _asbomber_man_game (Utilities|Casting|CastToBomberManGame (Game|GetGameMode)))
  (Default|OnBombermanCreatedEvent _asbomber_man_game self))

(event EventActorBeginOverlap
  (params (OtherActor :type Actor%20Object%20Reference)))

(event EventTick
  (params (DeltaSeconds :type Float%20%28single-precision%29)))

(event Collision|EventActorBeginOverlap
  (params (OtherActor :type Actor%20Object%20Reference))
  (Utilities|Casting|CastToBlueprint_Effect_Explosion OtherActor
    (:then
      (Game|Damage|ApplyDamage self 1e+02 0 0))
    (:CastFailed
      (bind _aspower_up_interface (Utilities|Casting|CastToPowerUpInterface OtherActor))
      (bind _type (Default|GetPowerUpType _aspower_up_interface))
      (bind _asbomberman_game_instance (Utilities|Casting|CastToBombermanGameInstance (Game|GetGameInstance)))
      (Default|AddPowerUp _asbomberman_game_instance _type))))

(fn ConstructionScript)