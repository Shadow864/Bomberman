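; Bomberman level actor that builds the tile grid, spawns the player and serves grid queries.
; The construction script loads tile data into instanced floor, solid and destroyable wall meshes and records the player spawn.
; BeginPlay registers the map with the game mode, and the first Tick spawns the character.
; Helpers convert grid and world positions, trace for empty tiles, cap bomb spawns by Extra Bomb count and map tiles to exit or power-up classes.
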(event EventBeginPlay
  (bind _asbomber_man_game (Utilities|Casting|CastToBomberManGame (Game|GetGameMode)))
  (Variables|/Game/Blueprints/BomberManGame.BomberManGame_C|SetMap _asbomber_man_game self)
  (Variables|Default|SetGameMode _asbomber_man_game)
  (bind _asbomberman_game_instance (Utilities|Casting|CastToBombermanGameInstance (Game|GetGameInstance)))
  (Variables|Default|SetGameInstance _asbomberman_game_instance))

(event EventActorBeginOverlap
  (params (OtherActor :type Actor%20Object%20Reference)))

(event EventTick
  (params (DeltaSeconds :type Float%20%28single-precision%29))
  (if (not (Variables|Default|GetSpawned))
    (Variables|Default|SetSpawned true)
    (Game|SpawnActorfromClass "/Game/Blueprints/Player/BombermanCharacter.BombermanCharacter_C" (Variables|Default|GetSpawnPoint) "Undefined" 0 0)))

(fn ConstructionScript
  (bind _tilesize (Variables|Default|GetTileSize))
  (bind (_width _height) (Utilities|Struct|BreakSize _tilesize))
  (CallFunction|LoadMap self)
  (for _array_element (Variables|Default|GetTilesInfo)
    (Components|InstancedStaticMesh|AddInstance (Variables|Default|GetFloor) (Math|Conversions|ToTransform(Vector) (Math|Vector|MakeVector (* (.X (Utilities|Struct|BreakPosition2D (.Position (Utilities|Struct|BreakTileInfo _array_element)))) (Math|Conversions|ToFloat(Integer) _width)) (* (.Y (Utilities|Struct|BreakPosition2D (.Position (Utilities|Struct|BreakTileInfo _array_element)))) (Math|Conversions|ToFloat(Integer) _height)) 0.0)))
    (switch Utilities|FlowControl|Switch|SwitchonTileType (.Type (Utilities|Struct|BreakTileInfo _array_element))
      (:NewEnumerator1
        (Components|InstancedStaticMesh|AddInstance (Variables|Default|GetSolidWall) (Math|Conversions|ToTransform(Vector) (Math|Vector|MakeVector (* (.X (Utilities|Struct|BreakPosition2D (.Position (Utilities|Struct|BreakTileInfo _array_element)))) (Math|Conversions|ToFloat(Integer) _width)) (* (.Y (Utilities|Struct|BreakPosition2D (.Position (Utilities|Struct|BreakTileInfo _array_element)))) (Math|Conversions|ToFloat(Integer) _height)) 0.0))))
      (:NewEnumerator2
        (Components|InstancedStaticMesh|AddInstance (Variables|Default|GetDestoyableWall) (Math|Conversions|ToTransform(Vector) (Math|Vector|MakeVector (* (.X (Utilities|Struct|BreakPosition2D (.Position (Utilities|Struct|BreakTileInfo _array_element)))) (Math|Conversions|ToFloat(Integer) _width)) (* (.Y (Utilities|Struct|BreakPosition2D (.Position (Utilities|Struct|BreakTileInfo _array_element)))) (Math|Conversions|ToFloat(Integer) _height)) 0.0))))
      (:NewEnumerator4
        (Variables|Default|SetSpawnPoint (Math|Conversions|ToTransform(Vector) (+ (CallFunction|ToWorldPosition (.Position (Utilities|Struct|BreakTileInfo _array_element))) "0, 0,90.000000")))))))

(fn IsEmpty
  (params (Position :type Position%202D%20Structure))
  (bind _result (CallFunction|ToWorldPosition Position))
  (bind _returnvalue (Collision|LineTraceByChannel (+ _result "0,0.000000,200.000000") (+ _result "0,0.000000,1.000000") "TraceTypeQuery1" true 0 "ForOneFrame" false))
  (return (not _returnvalue)))

(fn SpawnBomb
  (params (Position :type Position%202D%20Structure))
  (bind (_x _y) (Utilities|Struct|BreakPosition2D Position))
  (bind _tilesize (Variables|Default|GetTileSize))
  (bind (_width _height) (Utilities|Struct|BreakSize _tilesize))
  (bind _count (Default|GetPowerUpCount (Variables|Default|GetGameInstance) "NewEnumerator2"))
  (if (< (Variables|/Game/Blueprints/BomberManGame.BomberManGame_C|GetBombs (Variables|Default|GetGameMode)) _count)
    (Game|SpawnActorfromClass "/Game/Blueprints/Level/Bomb.Bomb_C" (Math|Conversions|ToTransform(Vector) (Math|Vector|MakeVector (Math|Conversions|ToFloat(Integer) (* _x _width)) (Math|Conversions|ToFloat(Integer) (* _y _height)) 0.0)) "Undefined" 0 0)))

(fn ToWorldPosition
  (params (Position :type Position%202D%20Structure))
  (bind (_x _y) (Utilities|Struct|BreakPosition2D Position))
  (bind _tilesize (Variables|Default|GetTileSize))
  (bind (_width _height) (Utilities|Struct|BreakSize _tilesize))
  (return (Math|Vector|MakeVector (Math|Conversions|ToFloat(Integer) (* _x _width)) (Math|Conversions|ToFloat(Integer) (* _y _height)) 0.0)))

(fn GetSpawnClassfromTile
  (params (Tile :type Tile%20Info%20Structure))
  (bind (_type _position _powerup _exit) (Utilities|Struct|BreakTileInfo Tile))
  (if _exit
    (return false "/Game/Blueprints/Level/Exit.Exit_C")
    (else
      (switch Utilities|FlowControl|Switch|SwitchonPowerUpType _powerup
        (:NewEnumerator0
          (return false "/Game/Blueprints/PowerUps/PowerUp_Accelerator.PowerUp_Accelerator_C"))
        (:NewEnumerator1
          (return false "/Game/Blueprints/PowerUps/PowerUpExplosionExpander.PowerUpExplosionExpander_C"))
        (:NewEnumerator2
          (return false "/Game/Blueprints/PowerUps/PowerUpExtraBomb.PowerUpExtraBomb_C"))
        (:NewEnumerator3
          (return false "/Game/Blueprints/PowerUps/PowerUpRemote.PowerUpRemote_C"))
        (:NewEnumerator4
          (return true 0))))))

(fn ToLocalPosition
  (params (WorldPosition :type Position%202D%20Structure))
  (bind (_x _y) (Utilities|Struct|BreakPosition2D WorldPosition))
  (bind _tilesize (Variables|Default|GetTileSize))
  (bind _tilesize_2 (Variables|Default|GetTileSize))
  (bind (_width _height) (Utilities|Struct|BreakSize _tilesize_2))
  (bind (_width_2 _height_2) (Utilities|Struct|BreakSize _tilesize))
  (return (Utilities|Struct|MakePosition2D (/ (+ _x (/ _width_2 2)) _width) (/ (+ (/ _height_2 2) _y) _height))))

(fn ToIndexLocalPosition
  (params (Position :type Position%202D%20Structure))
  (bind (_x _y) (Utilities|Struct|BreakPosition2D Position))
  (return (+ _x (* _y (.Width (Utilities|Struct|BreakSize (Variables|Default|GetMapSize)))))))