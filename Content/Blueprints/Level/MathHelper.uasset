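; MathHelper is a set of helper functions for a Position2D struct with X and Y components.
; It compares two positions for exact component equality, adds them component-wise, and converts a Left, Right, Top or Down direction into a unit Position2D offset.
; X is the Top/Down axis and Y is the Left/Right axis, with Top and Right positive.
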(fn Equal
  (params (A :type Position%202D%20Structure) (B :type Position%202D%20Structure))
  (bind (_x _y) (Utilities|Struct|BreakPosition2D A))
  (bind (_x_2 _y_2) (Utilities|Struct|BreakPosition2D B))
  (return (and (== _x _x_2) (== _y _y_2))))

(fn Position2d+Position2d
  (params (A :type Position%202D%20Structure) (B :type Position%202D%20Structure))
  (bind (_x _y) (Utilities|Struct|BreakPosition2D A))
  (bind (_x_2 _y_2) (Utilities|Struct|BreakPosition2D B))
  (return (Utilities|Struct|MakePosition2D (+ _x _x_2) (+ _y _y_2))))

(fn GetDirectionVector
  (params (A :type Direction%20Enum))
  (switch Utilities|FlowControl|Switch|SwitchonDirection A
    (:NewEnumerator0
      (return (Utilities|Struct|MakePosition2D 0 -1)))
    (:NewEnumerator1
      (return (Utilities|Struct|MakePosition2D 0 1)))
    (:NewEnumerator2
      (return (Utilities|Struct|MakePosition2D 1)))
    (:NewEnumerator3
      (return (Utilities|Struct|MakePosition2D -1)))))