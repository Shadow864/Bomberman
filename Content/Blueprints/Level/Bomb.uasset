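; Bomberman bomb actor that pulses its mesh through a Scale timeline and explodes after a delay.
; It spawns explosion effects tile by tile in each direction, with reach set by a GameInstance power-up count, stopping after a vertical trace hits.
; Overlapping another explosion detonates it after a short delay, chaining bombs, with an Exploded flag preventing repeats.
; It reports creation from the construction script and destruction to the BomberManGame mode.
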(event EventBeginPlay
  (bind _scale (Timeline|Scale Play)
    (:Update
      (Transformation|SetWorldScale3D (Variables|Default|GetStaticMesh) (Math|Conversions|ToVector(Float) _scale))
      (bind _asbomberman_game_instance (Utilities|Casting|CastToBombermanGameInstance (Game|GetGameInstance)))
      (bind _output_get (Variables|Default|SetGameInstance _asbomberman_game_instance))
      (bind _count (Default|GetPowerUpCount _output_get "NewEnumerator1"))
      (Variables|Default|SetForce _count)
      (Utilities|FlowControl|Delay (Variables|Default|GetExplosionDelay))
      (if (not (Variables|Default|GetExploded))
        (Variables|Default|SetExploded true)
        (Game|SpawnActorfromClass "/Game/StarterContent/Blueprints/Blueprint_Effect_Explosion.Blueprint_Effect_Explosion_C" (Math|Conversions|ToTransform(Vector) (Transformation|GetActorLocation)) "AlwaysSpawn" 0 0)
        (Utilities|FlowControl|Delay 0.0)
        (bind _enumvalue (|ForEachDirection)
          (:LoopBody
            (CallFunction|SpawnExplosions (Transformation|GetActorLocation) 0 _enumvalue 100))
          (:then
            (Actor|DestroyActor)))))))

(event EventActorBeginOverlap
  (params (OtherActor :type Actor%20Object%20Reference)))

(event EventTick
  (params (DeltaSeconds :type Float%20%28single-precision%29)))

(event Collision|EventActorBeginOverlap
  (params (OtherActor :type Actor%20Object%20Reference))
  (Utilities|FlowControl|Delay 0.5)
  (Utilities|Casting|CastToBlueprint_Effect_Explosion OtherActor)
  (if (not (Variables|Default|GetExploded))
    (Variables|Default|SetExploded true)
    (Game|SpawnActorfromClass "/Game/StarterContent/Blueprints/Blueprint_Effect_Explosion.Blueprint_Effect_Explosion_C" (Math|Conversions|ToTransform(Vector) (Transformation|GetActorLocation)) "AlwaysSpawn" 0 0)
    (Utilities|FlowControl|Delay 0.0)
    (bind _enumvalue (|ForEachDirection)
      (:LoopBody
        (CallFunction|SpawnExplosions (Transformation|GetActorLocation) 0 _enumvalue 100))
      (:then
        (Actor|DestroyActor)))))

(event EventDestroyed
  (bind _asbomber_man_game (Utilities|Casting|CastToBomberManGame (Game|GetGameMode)))
  (Default|OnBombDestroyedEvent _asbomber_man_game self))

(fn ConstructionScript
  (bind _asbomber_man_game (Utilities|Casting|CastToBomberManGame (Game|GetGameMode)))
  (Default|OnBombCreatedEvent _asbomber_man_game self))

(fn GetDirectionVector
  (params (Direction :type Direction%20Enum))
  (switch Utilities|FlowControl|Switch|SwitchonDirection Direction
    (:NewEnumerator0
      (return "0,-1.000000,0"))
    (:NewEnumerator1
      (return "0,1.000000,0"))
    (:NewEnumerator2
      (return "-1.000000,0,0"))
    (:NewEnumerator3
      (return "1.000000,0,0"))))

(fn SpawnExplosions
  (params (Center :type Vector) (Delay :type Integer) (Direction :type Direction%20Enum) (TileSize :type Integer))
  (bind _index (Utilities|FlowControl|ForLoopwithBreak 0 (+ (Variables|Default|GetForce) 1) :!label _label)
    (:LoopBody
      (bind _returnvalue (Collision|LineTraceByChannel (+ (+ Center (* (CallFunction|GetDirectionVector Direction) (* TileSize _index))) "0,0.000000,100.000000") (+ "0, 0,10.000000" (+ Center (* (CallFunction|GetDirectionVector Direction) (* TileSize _index)))) "TraceTypeQuery1" false 0 "ForDuration"))
      (Game|SpawnActorfromClass "/Game/StarterContent/Blueprints/Blueprint_Effect_Explosion.Blueprint_Effect_Explosion_C" (Math|Conversions|ToTransform(Vector) (+ Center (* (CallFunction|GetDirectionVector Direction) (* TileSize _index)))) "AlwaysSpawn" 0 0)
      (if _returnvalue
        (goto _label Break)))))