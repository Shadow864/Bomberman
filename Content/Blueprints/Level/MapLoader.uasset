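; MapLoader procedurally builds a tile grid for a given map from its size and stores it in the map's TilesInfo.
; LoadMap fills a flat, column-major array, deriving each X/Y position from the index and the map height.
; GetTileType sets the type by rule: one enum value for the border and even/even interior pillars, a special one at (1,1), and a default elsewhere.
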(fn LoadMap
  (params (Map :type Map%20Object%20Reference))
  (bind _mapsize (Variables|/Game/Blueprints/Level/Map.Map_C|GetMapSize Map))
  (bind (_width _height) (Utilities|Struct|BreakSize _mapsize))
  (bind _returnvalue (* _width _height))
  (Utilities|Array|Resize (LocalVariables|GetTiles) _returnvalue)
  (for _index (range 0 (- _returnvalue 1))
    (Utilities|Array|SetArrayElem (LocalVariables|GetTiles) _index (Utilities|Struct|MakeTileInfo (CallFunction|GetTileType (Utilities|Struct|MakePosition2D (/ _index _height) (Math|Integer|%(Integer) _index _height)) _mapsize) (Utilities|Struct|MakePosition2D (/ _index _height) (Math|Integer|%(Integer) _index _height)) "NewEnumerator0" false))
    (Variables|/Game/Blueprints/Level/Map.Map_C|SetTilesInfo Map (LocalVariables|GetTiles))))

(fn GetTileType
  (params (Position :type Position%202D%20Structure) (Size :type Size%20Structure))
  (bind (_x _y) (Utilities|Struct|BreakPosition2D Position))
  (bind (_width _height) (Utilities|Struct|BreakSize Size))
  (if (and (== _x 1) (== _y 1))
    (return "NewEnumerator4")
    (elif (Math|Boolean|ORBoolean (== _x 0) (== _x (- _width 1)) (== _y 0) (== _y (- _height 1)) (and (== (Math|Integer|%(Integer) _x 2) 0) (== (Math|Integer|%(Integer) _y 2) 0)))
      (return "NewEnumerator1")
      (else
        (return "NewEnumerator0")))))