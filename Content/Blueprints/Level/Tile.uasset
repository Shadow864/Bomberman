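; Tile is a level grid cell actor that displays a floor with an optional solid or destroyable wall.
; ChangeType stores the tile type enum and calls Refrash, which shows the matching wall component and always keeps the floor visible.
; Only component visibility changes, with no collision handling, and the event graph and construction script are empty.
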(event EventBeginPlay)

(event EventActorBeginOverlap
  (params (OtherActor :type Actor%20Object%20Reference)))

(event EventTick
  (params (DeltaSeconds :type Float%20%28single-precision%29)))

(fn ConstructionScript)

(fn ChangeType
  (params (Type :type TileType%20Enum))
  (Variables|Default|SetType Type)
  (CallFunction|Refrash))

(fn Refrash
  (Rendering|SetVisibility (Variables|Default|GetWallSolid) (Utilities|Enum|Equal(Enum) (Variables|Default|GetType) "NewEnumerator1") false)
  (Rendering|SetVisibility (Variables|Default|GetWallDestroyable) (Utilities|Enum|Equal(Enum) (Variables|Default|GetType) "NewEnumerator2") false)
  (Rendering|SetVisibility (Variables|Default|GetFloor) true false))